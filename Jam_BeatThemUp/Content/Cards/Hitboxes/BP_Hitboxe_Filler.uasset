(event Custom|AttackFrame
  (CallFunction|SpawnHitboxe (Variables|Default|GetBox) (Variables|Default|GetHitboxeSize))
  (Utilities|FlowControl|Delay 0.0)
  (CallFunction|SpawnHitboxe (Variables|Default|GetBox1) (Variables|Default|GetHitboxeSize_1))
  (Utilities|FlowControl|Delay 0.0)
  (CallFunction|SpawnHitboxe (Variables|Default|GetBox2) (Variables|Default|GetHitboxeSize_2)))

(event Custom|StopAttackFrame
  (Utilities|Time|ClearandInvalidateTimerbyHandle (stale EventBeginPlay _returnvalue_3))
  (if (not (> (Utilities|Array|Length (Variables|Default|GetNPC_AlreadyHited)) 0))
    (Default|EventMiss (CallFunction|GetBPPlayer))
    (Actor|DestroyActor)))

(event EventBeginPlay
  (Components|Timeline|SetLooping (Variables|Default|GetPaperFlipbook) false)
  (bind _returnvalue (Actor|GetActorOfClass "/Game/Assets/Sound_Design/BP_Sound_a_intégrer.BP_Sound_a_intégrer_C"))
  (Default|FillerExplosion _returnvalue)
  (switch Utilities|FlowControl|Switch|SwitchonE_Family (Variables|Default|GetFamily)
    (:NewEnumerator0
      (Sprite|SetFlipbook (Variables|Default|GetPaperFlipbook) "/Game/Root/VFX/Filler/Earth/FillerEarthFlipBook.FillerEarthFlipBook"))
    (:NewEnumerator1
      (Sprite|SetFlipbook (Variables|Default|GetPaperFlipbook) "/Game/Root/VFX/Filler/Fire/FillerFireFlipBook.FillerFireFlipBook" :!label _label))
    (:NewEnumerator2
      (goto _label))
    (:NewEnumerator3
      (Sprite|SetFlipbook (Variables|Default|GetPaperFlipbook) "/Game/Root/VFX/Filler/Thunder/FillerThunderFlipBook.FillerThunderFlipBook")))
  (bind _returnvalue_2 (Utilities|GetDataTableRow "/Game/Cards/Master/DT_Cards.DT_Cards" (Variables|Default|GetCardName))
    (:then
      (Audio|Components|Audio|Play (Variables|Default|GetPaperFlipbook))
      (Variables|Default|SetIDCard _returnvalue_2)
      (bind _returnvalue_3 (Utilities|Time|SetTimerbyEvent (delegate Custom|AttackFrame) 0.25 true))
      (Utilities|Time|SetTimerbyEvent (delegate Custom|StopAttackFrame) (.Duration (Utilities|Struct|BreakF_Card _returnvalue_2))))))

(event EventHitboxLoop
  (params (ArrayElement :type Hit%20Result%20Structure) (ArrayIndex :type Integer))
  (bind _npc_alreadyhited (Variables|Default|GetNPC_AlreadyHited))
  (bind _asbp_iamaster (Utilities|Casting|CastToBP_IAMaster (.HitActor (Collision|BreakHitResult ArrayElement))))
  (bind _returnvalue (Utilities|GetDataTableRow "/Game/Cards/Master/DT_Cards.DT_Cards" (Variables|Default|GetCardName))
    (:then
      (bind _output_get (Variables|Default|SetNPC_Hited _asbp_iamaster))
      (if (not (Utilities|Array|ContainsItem _npc_alreadyhited _output_get))
        (Utilities|Array|Add _npc_alreadyhited _output_get)
        (Default|GetHit _asbp_iamaster (.Damage (Utilities|Struct|BreakF_Card _returnvalue)) (Variables|Default|GetIDCard))
        (Utilities|FlowControl|Sequence
          (:then_0
            (Utilities|FlowControl|DoOnce false
              (:Completed
                (Default|EventHIT (CallFunction|GetBPPlayer) (Variables|Default|GetFamily)))))
          (:then_1
            (Default|EventEnemygotHit (CallFunction|GetBPPlayer))))))))

(fn ConstructionScript
  (Variables|Default|SetHitboxeSize (Variables|/Script/Engine.BoxComponent|GetBoxExtent (Variables|Default|GetBox)))
  (Variables|Default|SetHitboxeSize_1 (Variables|/Script/Engine.BoxComponent|GetBoxExtent (Variables|Default|GetBox1)))
  (Variables|Default|SetHitboxeSize_2 (Variables|/Script/Engine.BoxComponent|GetBoxExtent (Variables|Default|GetBox1))))