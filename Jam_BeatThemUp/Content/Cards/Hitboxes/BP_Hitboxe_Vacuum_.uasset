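; Card hitbox for a vacuum effect that pulls AI enemies toward its first box and damages them.
; On BeginPlay it spawns timed, repeated hitboxes through four boxes in sequence using a delayed for-loop macro, with the extra boxes' sizes cached in the construction script.
; Each BP_IAMaster hit is launched toward the first box on Y and Z only, then takes the card's damage from DT_Cards.
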(event EventBeginPlay
  (|CallParentFunction)
  (Utilities|ForLoopDelay 0 (Variables|Default|GetNbr_Tick) (Variables|Default|GetTick_delay)
    (:LoopBody
      (CallFunction|SpawnHitboxe (Variables|Default|GetBox) (Variables|Default|GetHitboxeSize)))
    (:Completed
      (Utilities|FlowControl|Delay 0.0)
      (Utilities|ForLoopDelay 0 (Variables|Default|GetNbr_Tick) (Variables|Default|GetTick_delay)
        (:LoopBody
          (CallFunction|SpawnHitboxe (Variables|Default|GetBox1) (Variables|Default|GetHitboxeSize_1)))
        (:Completed
          (Utilities|FlowControl|Delay 0.0)
          (Utilities|ForLoopDelay 0 (Variables|Default|GetNbr_Tick) (Variables|Default|GetTick_delay)
            (:LoopBody
              (CallFunction|SpawnHitboxe (Variables|Default|GetBox2) (Variables|Default|GetHitboxeSize_2)))
            (:Completed
              (Utilities|FlowControl|Delay 0.0)
              (Utilities|ForLoopDelay 0 (Variables|Default|GetNbr_Tick) (Variables|Default|GetTick_delay)
                (:LoopBody
                  (CallFunction|SpawnHitboxe (Variables|Default|GetBox3) (Variables|Default|GetHitboxeSize_3)))))))))))

(event EventHitboxLoop
  (params (ArrayElement :type Hit%20Result%20Structure) (ArrayIndex :type Integer))
  (bind _returnvalue (Math|Conversions|ToVector(Float) 5e+02))
  (bind _hitactor (Collision|BreakHitResult ArrayElement))
  (bind _box (Variables|Default|GetBox))
  (bind _returnvalue_2 (Transformation|GetActorLocation _hitactor))
  (bind _returnvalue_3 (Transformation|GetWorldLocation _box))
  (bind _returnvalue_4 (Math|Vector|GetUnitDirection(Vector) _returnvalue_2 _returnvalue_3))
  (bind _returnvalue_5 (* _returnvalue_4 _returnvalue))
  (bind _asbp_iamaster (Utilities|Casting|CastToBP_IAMaster _hitactor))
  (Character|LaunchCharacter _asbp_iamaster (Math|Vector|MakeVector 0.0 (.y _returnvalue_5) (.z _returnvalue_5)) true true)
  (bind _returnvalue_6 (Utilities|GetDataTableRow "/Game/Cards/Master/DT_Cards.DT_Cards" (Variables|Default|GetCardName))
    (:then
      (Default|GetHit _asbp_iamaster (.Damage (Utilities|Struct|BreakF_Card _returnvalue_6))))))

(fn ConstructionScript
  (|CallParentFunction)
  (Variables|Default|SetHitboxeSize_1 (Variables|/Script/Engine.BoxComponent|GetBoxExtent (Variables|Default|GetBox1)))
  (Variables|Default|SetHitboxeSize_2 (Variables|/Script/Engine.BoxComponent|GetBoxExtent (Variables|Default|GetBox2)))
  (Variables|Default|SetHitboxeSize_3 (Variables|/Script/Engine.BoxComponent|GetBoxExtent (Variables|Default|GetBox3))))