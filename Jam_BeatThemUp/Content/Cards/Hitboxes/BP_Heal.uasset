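; BP_Heal is a card effect actor that heals the player as soon as it spawns.
; BeginPlay adds a fixed amount to BP_Player's ActualLife with no clamp, then removes two entries from GI_Jam's ADeck, looked up at hard-coded indices.
; It then has the game instance create two cards and add them to the pull, a short delay apart.
; Overlap and Tick are unused.
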(event EventBeginPlay
  (|CallParentFunction)
  (bind _asbp_player (Utilities|Casting|CastToBP_Player (Game|GetPlayerCharacter 0)))
  (Variables|/Game/Root/GD/Player/BP_Player.BP_Player_C|SetActualLife _asbp_player (+ (Variables|/Game/Root/GD/Player/BP_Player.BP_Player_C|GetActualLife _asbp_player) 2))
  (bind _asgi_jam (Utilities|Casting|CastToGI_Jam (Game|GetGameInstance)))
  (Utilities|Array|RemoveItem (Variables|/Game/Root/GD/GI_Jam.GI_Jam_C|GetA_Deck _asgi_jam) (Utilities|Array|Get(acopy) (Variables|/Game/Root/GD/GI_Jam.GI_Jam_C|GetA_Deck _asgi_jam) 2))
  (Utilities|Array|RemoveItem (Variables|/Game/Root/GD/GI_Jam.GI_Jam_C|GetA_Deck _asgi_jam) (Utilities|Array|Get(acopy) (Variables|/Game/Root/GD/GI_Jam.GI_Jam_C|GetA_Deck _asgi_jam) 3))
  (bind _out_row (Default|CreateCard _asgi_jam))
  (Default|AddCardinPull _asgi_jam _out_row)
  (Utilities|FlowControl|Delay 0.25)
  (bind _out_row_2 (Default|CreateCard _asgi_jam))
  (Default|AddCardinPull _asgi_jam _out_row_2))

(event Collision|EventActorBeginOverlap
  (params (OtherActor :type Actor%20Object%20Reference)))

(event EventTick
  (params (DeltaSeconds :type Float%20%28single-precision%29)))

(fn ConstructionScript
  (|CallParentFunction))