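; Finisher card hitbox that damages AI characters it hits and slams them straight down.
; On BeginPlay it spawns six box hitboxes in sequence with zero-length delays between them, with five sizes cached from box extents in the construction script.
; For each hit, it reads damage from DT_Cards by card name, calls GetHit on BP_IAMaster targets and launches them downward, overriding existing velocity.
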(event EventHitboxLoop
  (params (ArrayElement :type Hit%20Result%20Structure) (ArrayIndex :type Integer))
  (bind _returnvalue (Utilities|GetDataTableRow "/Game/Cards/Master/DT_Cards.DT_Cards" (Variables|Default|GetCardName))
    (:then
      (bind _asbp_iamaster (Utilities|Casting|CastToBP_IAMaster (.HitActor (Collision|BreakHitResult ArrayElement))))
      (Default|GetHit _asbp_iamaster (.Damage (Utilities|Struct|BreakF_Card _returnvalue)))
      (Character|LaunchCharacter _asbp_iamaster "0, 0,-1000.000000" true true))))

(event EventBeginPlay
  (|CallParentFunction)
  (CallFunction|SpawnHitboxe (Variables|Default|GetBox) (Variables|Default|GetHitboxeSize))
  (Utilities|FlowControl|Delay 0.0)
  (CallFunction|SpawnHitboxe (Variables|Default|GetBox1) (Variables|Default|GetHitboxeSize_1))
  (Utilities|FlowControl|Delay 0.0)
  (CallFunction|SpawnHitboxe (Variables|Default|GetBox2) (Variables|Default|GetHitboxeSize_2))
  (Utilities|FlowControl|Delay 0.0)
  (CallFunction|SpawnHitboxe (Variables|Default|GetBox3) (Variables|Default|GetHitboxeSize_3))
  (Utilities|FlowControl|Delay 0.0)
  (CallFunction|SpawnHitboxe (Variables|Default|GetBox4) (Variables|Default|GetHitboxeSize_4))
  (Utilities|FlowControl|Delay 0.0)
  (CallFunction|SpawnHitboxe (Variables|Default|GetBox5) (Variables|Default|GetHitboxeSize_5))
  (Utilities|FlowControl|Delay 0.0))

(fn ConstructionScript
  (|CallParentFunction)
  (Variables|Default|SetHitboxeSize_1 (Variables|/Script/Engine.BoxComponent|GetBoxExtent (Variables|Default|GetBox1)))
  (Variables|Default|SetHitboxeSize_2 (Variables|/Script/Engine.BoxComponent|GetBoxExtent (Variables|Default|GetBox2)))
  (Variables|Default|SetHitboxeSize_3 (Variables|/Script/Engine.BoxComponent|GetBoxExtent (Variables|Default|GetBox3)))
  (Variables|Default|SetHitboxeSize_4 (Variables|/Script/Engine.BoxComponent|GetBoxExtent (Variables|Default|GetBox4)))
  (Variables|Default|SetHitboxeSize_5 (Variables|/Script/Engine.BoxComponent|GetBoxExtent (Variables|Default|GetBox5))))