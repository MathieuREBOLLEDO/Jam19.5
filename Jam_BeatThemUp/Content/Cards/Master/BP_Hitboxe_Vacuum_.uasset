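; BP_Hitboxe_Vacuum_ is a card hitbox Blueprint that spawns four boxes when play begins.
; After the parent BeginPlay, it calls SpawnHitboxe for each box with its own size, separated by zero-second delays.
; An unconnected chain, which never runs, would apply radial force from a box and deal the card's DT_Cards damage to hit BP_IAMaster actors.
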(event EventBeginPlay
  (|CallParentFunction)
  (CallFunction|SpawnHitboxe (Variables|Default|GetBox) (Variables|Default|GetHitboxeSize))
  (Utilities|FlowControl|Delay 0.0)
  (CallFunction|SpawnHitboxe (Variables|Default|GetBox1) (Variables|Default|GetHitboxeSize_1))
  (Utilities|FlowControl|Delay 0.0)
  (CallFunction|SpawnHitboxe (Variables|Default|GetBox2) (Variables|Default|GetHitboxeSize_2))
  (Utilities|FlowControl|Delay 0.0)
  (CallFunction|SpawnHitboxe (Variables|Default|GetBox3) (Variables|Default|GetHitboxeSize_3)))

(fn ConstructionScript
  (|CallParentFunction))