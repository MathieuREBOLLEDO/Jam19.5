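; AC_card_master is a master card component that spawns hitbox actors for cards in the game.
; SpawnHitboxes looks up its RowName in DT_Cards and always spawns that row's Hitboxes class at player 0's location.
; It stores the spawned actor and calls a named timer for DestroyHitboxes with no duration set.
; DestroyHitboxes destroys the stored actor and prints a debug string.
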(fn SpawnHitboxes
  (bind _returnvalue (Utilities|GetDataTableRow "/Game/Cards/Master/DT_Cards.DT_Cards" (Variables|Default|GetRowName))
    (:then
      (bind _returnvalue_2 (Game|SpawnActorfromClass (Utilities|Struct|BreakF_Card _returnvalue) (Math|Transform|MakeTransform (.location (Transformation|GetActorTransform (Game|GetPlayerCharacter 0))) "0, 0, 0" "1.000000,1.000000,1.000000") "AlwaysSpawn" 0 0))
      (Variables|Default|SetHitboxe _returnvalue_2)
      (Utilities|Time|SetTimerbyFunctionName 0 "DestroyHitboxes" 0.0))))

(fn DestroyHitboxes
  (Actor|DestroyActor (Variables|Default|GetHitboxe))
  (Development|PrintString "Hello"))