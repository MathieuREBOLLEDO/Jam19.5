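; BP_Hitboxe_Master is a master hitbox Blueprint in the Cards folder that runs a box overlap check when play begins.
; The construction script copies the Box component's extent into HitboxeSize, which BeginPlay passes to SpawnHitboxe with the Box.
; SpawnHitboxe does a zero-length multi box trace on the Visibility channel with debug drawing.
; It returns on the first hit, and BeginPlay leaves the result unused.
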(event EventBeginPlay
  (CallFunction|SpawnHitboxe (Variables|Default|GetBox) (Variables|Default|GetHitboxeSize)))

(fn ConstructionScript
  (Variables|Default|SetHitboxeSize (Variables|/Script/Engine.BoxComponent|GetBoxExtent (Variables|Default|GetBox))))

(fn SpawnHitboxe
  (params (Hitbox :type Box%20Component%20Object%20Reference) (Size :type Vector))
  (bind _returnvalue (Transformation|GetWorldLocation Hitbox))
  (bind _outhits (Class|KismetSystemLibrary|BoxTraceMulti _returnvalue _returnvalue Size "0, 0, 0" "TraceTypeQuery1" false 0 "ForDuration" true))
  (for (_array_element _array_index) _outhits
    (return false _array_element _array_index)))