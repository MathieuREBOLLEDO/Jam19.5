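; BP_Card_Master is a master Blueprint for cards, with its data held in a CardStruct.
; On BeginPlay it calls a Debug function, which prints the card's name, damage, level and family when the struct's Debug flag is set.
; It has no other gameplay logic, and its construction script is empty.
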(event EventBeginPlay
  (Utilities|Debug))

(fn ConstructionScript)