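; BP_Hitboxe_Filler is a card actor that spawns three hitboxes from its box components when play begins.
; The construction script caches box extents as hitbox sizes, with the third size also read from Box1 rather than Box2.
; BeginPlay passes each box and size to SpawnHitboxe, separated by zero-second delays, and prints the card's name, damage and family.
; The hit results returned by the spawn calls are unused.
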(event EventBeginPlay
  (bind _card_struct (Variables|Default|GetCard_Struct))
  (bind (_cardname _damage _level _familly) (Utilities|Struct|BreakF_Card _card_struct))
  (bind _array_element (CallFunction|SpawnHitboxe (Variables|Default|GetBox) (Variables|Default|GetHitboxeSize)))
  (Development|PrintString (Utilities|String|Append "Card name :  " (Utilities|String|EnumtoString _cardname) " Damage deal :  " (Utilities|String|ToString(Float) _damage) " Family : " (Utilities|String|EnumtoString _familly)))
  (Utilities|FlowControl|Delay 0.0)
  (CallFunction|SpawnHitboxe (Variables|Default|GetBox1) (Variables|Default|GetHitboxeSize_1))
  (Utilities|FlowControl|Delay 0.0)
  (CallFunction|SpawnHitboxe (Variables|Default|GetBox2) (Variables|Default|GetHitboxeSize_2)))

(event Collision|EventActorBeginOverlap
  (params (OtherActor :type Actor%20Object%20Reference)))

(event EventTick
  (params (DeltaSeconds :type Float%20%28single-precision%29)))

(fn ConstructionScript
  (Variables|Default|SetHitboxeSize (Variables|/Script/Engine.BoxComponent|GetBoxExtent (Variables|Default|GetBox)))
  (Variables|Default|SetHitboxeSize_1 (Variables|/Script/Engine.BoxComponent|GetBoxExtent (Variables|Default|GetBox1)))
  (Variables|Default|SetHitboxeSize_2 (Variables|/Script/Engine.BoxComponent|GetBoxExtent (Variables|Default|GetBox1))))