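; BP_Hitboxe_Vacuum is a card hitbox Blueprint that runs one-shot box overlap traces from four box components on BeginPlay.
; The construction script caches box extents, with Box3's size taken from Box2.
; SpawnHitboxe runs a zero-length, debug-drawn Visibility multi-trace per box, separated by zero-second delays.
; Hits pass to HitboxLoop, which only returns them, so no vacuum effect is implemented here.
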(event EventBeginPlay
  (CallFunction|SpawnHitboxe (Variables|Default|GetBox) (Variables|Default|GetHitboxeSize))
  (Utilities|FlowControl|Delay 0.0)
  (CallFunction|SpawnHitboxe (Variables|Default|GetBox1) (Variables|Default|GetHitboxeSize_1))
  (Utilities|FlowControl|Delay 0.0)
  (CallFunction|SpawnHitboxe (Variables|Default|GetBox2) (Variables|Default|GetHitboxeSize_2))
  (Utilities|FlowControl|Delay 0.0)
  (CallFunction|SpawnHitboxe (Variables|Default|GetBox3) (Variables|Default|GetHitboxeSize_3)))

(fn ConstructionScript
  (Variables|Default|SetHitboxeSize (Variables|/Script/Engine.BoxComponent|GetBoxExtent (Variables|Default|GetBox)))
  (Variables|Default|SetHitboxeSize_1 (Variables|/Script/Engine.BoxComponent|GetBoxExtent (Variables|Default|GetBox1)))
  (Variables|Default|SetHitboxeSize_2 (Variables|/Script/Engine.BoxComponent|GetBoxExtent (Variables|Default|GetBox2)))
  (Variables|Default|SetHitboxeSize_3 (Variables|/Script/Engine.BoxComponent|GetBoxExtent (Variables|Default|GetBox2))))

(fn SpawnHitboxe
  (params (Hitbox :type Box%20Component%20Object%20Reference) (Size :type Vector))
  (bind _returnvalue (Transformation|GetWorldLocation Hitbox))
  (bind _outhits (Class|KismetSystemLibrary|BoxTraceMulti _returnvalue _returnvalue Size "0, 0, 0" "TraceTypeQuery1" false 0 "ForDuration" true))
  (for (_array_element _array_index) _outhits
    (CallFunction|HitboxLoop _array_element _array_index))
  (return "" 0))

(fn HitboxLoop
  (params (Array%20Element1 :type Hit%20Result%20Structure) (Array%20Index1 :type Integer))
  (return Array%20Element1 Array%20Index1))