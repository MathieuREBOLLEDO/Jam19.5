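; AC_ComboSystem is a player combo component, still partly unfinished, that counts landed hits toward combo levels.
; HitLanded increments a token; reaching the threshold raises the combo level and resets the token to its base, while ComboOver zeroes the token.
; HitMissed clears the family combo only below two.
; The already-hit enemy check does nothing, and the same-family increment logic is disconnected.
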(event Custom|ComboOver
  (Variables|Default|SetClassicComboToken 0))

(event Custom|HitLanded
  (params (EnnemieAlreadyHit :type Array%20of%20Actor%20Object%20References) (NewEnnemieHit :type Array%20of%20Actor%20Object%20References))
  ;[0 0 0] GainComboPointAndComboTimer
  (bind _result (Math|Integer|IncrementInt (Variables|Default|GetClassicComboToken))
    (:%20%20
      (if (>= _result (Variables|Default|GetClassicComboThreshold))
        (Math|Integer|IncrementInt (Variables|Default|GetClassicComboLevel)
          (:%20%20
            (Variables|Default|SetClassicComboToken (Variables|Default|GetBase%20Classic%20Combo%20Token)))))
      ;[1 1 1] CheckIfEnemyGotHitWitAttack
      (if (Utilities|Array|ContainsItem EnnemieAlreadyHit (Utilities|Array|Get(acopy) NewEnnemieHit))
        _))))

(event Custom|HitMissed
  (if (not (>= (Variables|Default|GetFamilyCombo) 2))
    (Variables|Default|SetFamilyCombo 0)))

(event EventBeginPlay)

(event EventTick
  (params (DeltaSeconds :type Float%20%28single-precision%29)))