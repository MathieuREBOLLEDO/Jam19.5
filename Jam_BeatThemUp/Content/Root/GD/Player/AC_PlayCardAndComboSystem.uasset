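; Actor component for playing cards and tracking combos on the player, currently an unfinished skeleton.
; On BeginPlay it caches its owner and binds four press events (X, A, Y, B) from GCJam for card input.
; All four handlers are empty.
; Combo logic for points and card-family streaks exists only as disconnected nodes that never run.
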(event Custom|Start)

(event Custom|PressXEvent
  ;[1 1 1] PressCardsInput
)

(event Custom|PressBEvent
  ;[1 1 1] PressCardsInput
)

(event Custom|PressAEvent
  ;[1 1 1] PressCardsInput
)

(event Custom|PressYEvent
  ;[1 1 1] PressCardsInput
)

(event EventBeginPlay
  (bind _asgc_jam (CallFunction|GetGCJam))
  ;[1 0.03439 0.7938] BeginPlay
  (Variables|Default|SetOwner (Components|GetOwner))
  (EventDispatchers|BindEventtoPressX _asgc_jam (delegate Custom|PressXEvent))
  (EventDispatchers|BindEventtoPressA _asgc_jam (delegate Custom|PressAEvent))
  (EventDispatchers|BindEventtoPressY _asgc_jam (delegate Custom|PressYEvent))
  (EventDispatchers|BindEventtoPressB _asgc_jam (delegate Custom|PressBEvent)))

(event EventTick
  (params (DeltaSeconds :type Float%20%28single-precision%29)))