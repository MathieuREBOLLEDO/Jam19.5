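; Player component that activates played cards, spawning the matching attack hitbox and tracking card-family combos.
; PlayCard keeps or breaks the player's combo by comparing the card's family to the last one, then spawns a Launcher, Vacuum, Filler or Finisher hitbox at the card's distance.
; Only Launcher and Filler set the spawn rotation, so Vacuum and Finisher reuse the stored value.
; BeginPlay binds four face-button events, whose handlers are empty.
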(event Custom|PlayCard
  (params (CardPlay :type F%20Card%20Structure))
  (bind _asgi_jam (CallFunction|GetGIJam))
  (bind _asbp_player (CallFunction|GetBPPlayer))
  (bind (_returnvalue _returnvalue2) (|SpawnTransform (.distance CardPlay)))
  (bind _output_get (Variables|/Game/Root/GD/GI_Jam.GI_Jam_C|SetCurrentCardFamilly _asgi_jam (.familly CardPlay)))
  (if (Utilities|Enum|Equal(Enum) (Variables|/Game/Root/GD/GI_Jam.GI_Jam_C|GetLastCardFamilly _asgi_jam) _output_get)
    (Default|KeepCombo _asbp_player)
    (else
      (Default|BreakCombo _asbp_player)))
  (Development|PrintString (Utilities|String|EnumtoString (.familly CardPlay)) true true "(R=1.000000,G=0.036710,B=0.000000,A=1.000000)" 0.1)
  (switch Utilities|FlowControl|Switch|SwitchonE_CardName (.cardname CardPlay)
    (:NewEnumerator0
      (Variables|Default|SetRotateHitBox "0, 0, 0")
      (Game|SpawnActorfromClass "/Game/Cards/Hitboxes/BP_Hitboxe_Launcher.BP_Hitboxe_Launcher_C" (Math|Transform|MakeTransform _returnvalue (Variables|Default|GetRotateHitBox) "1.000000,1.000000,1.000000") "Undefined" 0 (.familly CardPlay) 0))
    (:NewEnumerator1
      (Game|SpawnActorfromClass "/Game/Cards/Hitboxes/BP_Hitboxe_Vacuum_.BP_Hitboxe_Vacuum__C" (Math|Transform|MakeTransform _returnvalue (Variables|Default|GetRotateHitBox) "1.000000,1.000000,1.000000") "Undefined" 0 (.familly CardPlay) 0))
    (:NewEnumerator2
      (Variables|Default|SetRotateHitBox _returnvalue2)
      (Game|SpawnActorfromClass "/Game/Cards/Hitboxes/BP_Hitboxe_Filler.BP_Hitboxe_Filler_C" (Math|Transform|MakeTransform _returnvalue (Variables|Default|GetRotateHitBox) "1.000000,1.000000,1.000000") "Undefined" 0 (.familly CardPlay) 0))
    (:NewEnumerator3
      (Game|SpawnActorfromClass "/Game/Cards/Hitboxes/BP_Hitbox_Finisher.BP_Hitbox_Finisher_C" (Math|Transform|MakeTransform _returnvalue (Variables|Default|GetRotateHitBox) "1.000000,1.000000,1.000000") "Undefined" 0 (.familly CardPlay) 0))))

(event Custom|PressXEvent
  ;[1 1 1] PressCardsInput
)

(event Custom|PressBEvent
  ;[1 1 1] PressCardsInput
)

(event Custom|PressAEvent
  ;[1 1 1] PressCardsInput
)

(event Custom|PressYEvent
  ;[1 1 1] PressCardsInput
)

(event EventBeginPlay
  (bind _asgc_jam (CallFunction|GetGCJam))
  ;[1 0.03439 0.7938] BeginPlay
  (Variables|Default|SetOwner (Components|GetOwner))
  (EventDispatchers|BindEventtoPressX _asgc_jam (delegate Custom|PressXEvent))
  (EventDispatchers|BindEventtoPressA _asgc_jam (delegate Custom|PressAEvent))
  (EventDispatchers|BindEventtoPressY _asgc_jam (delegate Custom|PressYEvent))
  (EventDispatchers|BindEventtoPressB _asgc_jam (delegate Custom|PressBEvent)))

(event EventTick
  (params (DeltaSeconds :type Float%20%28single-precision%29)))

(fn SetCardValues
  (params (Montage%20to%20Play :type Anim%20Montage%20Object%20Reference))
  (Variables|Default|SetMontage%20to%20Play Montage%20to%20Play))