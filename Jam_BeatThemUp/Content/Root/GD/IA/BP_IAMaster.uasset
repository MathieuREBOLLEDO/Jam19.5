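; Master enemy character for flipbook-based card combat, running a behavior tree that receives the player through its blackboard.
; Tick picks idle, run or falling flipbooks and flips facing by velocity, while Attack is an empty event.
; GetHit shows a card-family impact, flags the blackboard and applies hit-stop through CustomTimeDilation and a timeline.
; The card type then sets any knockback launch before damage leads to recovery or death.
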(event Custom|Attack
  ;[1 1 1] HitedLogic
)

(event Custom|GetHit
  (params (HitValue :type Float%20%28double-precision%29) (Card :type F%20Card%20Structure))
  (bind _impact (Variables|Default|GetImpact))
  (Variables|Default|SetHit%20Value HitValue)
  (Variables|Default|SetCardUsed Card)
  (Variables|Default|SetHited true)
  (Variables|Default|SetAttacking? false)
  ;[1 1 1] HitedLogic
  (Audio|PlaySound2D (Utilities|Select :Index (Math|Random|RandomIntegerinRange 0 2) :Option%200 "/Game/Root/Sounds/SoundWaves/Hit1.Hit1" :Option%201 "/Game/Root/Sounds/SoundWaves/Hit2.Hit2" :Option%202 "/Game/Root/Sounds/SoundWaves/Hit3.Hit3") 1.0 1.0 0.0 0 0)
  (switch Utilities|FlowControl|Switch|SwitchonE_Family (.Familly (Utilities|Struct|BreakF_Card Card))
    (:NewEnumerator0
      (Sprite|SetFlipbook (Variables|Default|GetImpact) "/Game/Root/GD/IA/Impact/Earth/ImpactEarthfLIP.ImpactEarthfLIP"))
    (:NewEnumerator1
      (Sprite|SetFlipbook _impact "/Game/Root/GD/IA/Impact/Fire/ImpactFireFlipBook.ImpactFireFlipBook" :!label _label))
    (:NewEnumerator2
      (goto _label))
    (:NewEnumerator3
      (Sprite|SetFlipbook _impact "/Game/Root/GD/IA/Impact/Thunder/ImpactThunderFlip.ImpactThunderFlip")))
  (AI|Components|Blackboard|SetValueasBool (AI|GetBlackboard (Pawn|GetController)) (Utilities|Name|MakeLiteralName "Hited?") true)
  (Audio|Components|Audio|Play (Variables|Default|GetImpact))
  (Sprite|SetFlipbook (Variables|Default|GetFlipBook) (Variables|Default|GetHitFlipBook))
  (Variables|Default|SetCustomTimeDilation 0.0) ; StartHitStop
  ;[1 1 1] Feeback Ennemy
  (Timeline|Timeline_1 PlayFromStart
    (:Finished
      (Variables|Default|SetCustomTimeDilation 1.0) ; End HitStop
      (Variables|/Script/Engine.CharacterMovementComponent|SetGroundFriction (Variables|Character|GetCharacterMovement) 0.0)
      (switch Utilities|FlowControl|Switch|SwitchonE_CardName (.CardName (Utilities|Struct|BreakF_Card (Variables|Default|GetCardUsed)))
        (:NewEnumerator0
          ;[1 1 1] LauncherBump
          (Character|LaunchCharacter (* (Transformation|GetActorUpVector) (.PowerLaunch (Utilities|Struct|BreakF_Card (Variables|Default|GetCardUsed)))) true true))
        (:NewEnumerator1
          _)
        (:NewEnumerator2
          (Character|LaunchCharacter (Math|Vector|MakeVector (.x (* (Math|Vector|NegateVector (Math|Vector|GetForwardVector (Variables|Collision|GetCapsuleComponent))) (.PowerLaunch (Utilities|Struct|BreakF_Card (Variables|Default|GetCardUsed))))) (.y (* (Math|Vector|NegateVector (Math|Vector|GetForwardVector (Variables|Collision|GetCapsuleComponent))) (.PowerLaunch (Utilities|Struct|BreakF_Card (Variables|Default|GetCardUsed))))) 2e+02) true true))
        (:NewEnumerator3
          ;[1 1 1] Finisher Bump/Smash
          (Character|LaunchCharacter (* (Transformation|GetActorUpVector) (Math|Float|SelectFloat (* (.PowerLaunch (Utilities|Struct|BreakF_Card (Variables|Default|GetCardUsed))) -1.0) (/ (.PowerLaunch (Utilities|Struct|BreakF_Card (Variables|Default|GetCardUsed))) 2.0) (AI|Components|NavMovement|IsFalling (Variables|Character|GetCharacterMovement)))) true true)))
      (Utilities|FlowControl|RetriggerableDelay (Variables|Default|GetDelayAnimationHited))
      ;[1 1 1] Death
      (bind _output_get (Variables|Default|SetHP (- (Variables|Default|GetHP) (Variables|Default|GetHit%20Value))))
      (if (<= _output_get 0.0)
        (Sprite|SetFlipbook (Variables|Default|GetFlipBook) (Variables|Default|GetDeathFlipBook))
        (Audio|PlaySound2D "/Game/Assets/Sound_Design/SFX/SFX_Goblin_Death_Cue.SFX_Goblin_Death_Cue" 1.0 1.0 0.0 0 0)
        (Utilities|FlowControl|Delay (Variables|Default|GetDelayAnimationDead))
        (Actor|DestroyActor)
        (else
          ;[1 1 1] ResetHited
          (Variables|Default|SetHited false)
          (AI|Components|Blackboard|SetValueasBool (AI|GetBlackboard (Pawn|GetController)) (Utilities|Name|MakeLiteralName "Hited?") false)
          (Utilities|FlowControl|Delay 0.2)
          (Variables|/Script/Engine.CharacterMovementComponent|SetGroundFriction (Variables|Character|GetCharacterMovement) 8.0))))))

(event EventBeginPlay
  (bind _self self)
  (bind _flipbook (Variables|Default|GetFlipBook))
  (bind _returnvalue (AI|GetAIController _self))
  (bind _relativelocation (Variables|/Script/Engine.SceneComponent|GetRelativeLocation _flipbook))
  ;[1 1 1] BeginPlay
  (Variables|Default|SetInitialPosition (Math|Vector|MakeVector (.x _relativelocation) (+ (.y _relativelocation) (Math|Random|RandomFloatinRange -5e+01 5e+01)) (.z _relativelocation)))
  ;;[1 1 1] SetBehaviorTreeAndPlayerToAI
  (AI|RunBehaviorTree _returnvalue (Variables|Default|GetBehaviorTreeAI))
  (AI|Components|Blackboard|SetValueasObject (AI|GetBlackboard _returnvalue) (Utilities|Name|MakeLiteralName "Player") (CallFunction|GetBPPlayer))
  (Components|Timeline|SetLooping (Variables|Default|GetImpact) false))

(event EventTick
  (params (DeltaSeconds :type Float%20%28single-precision%29))
  (bind _returnvalue (Transformation|GetActorLocation))
  (Utilities|FlowControl|Sequence
    (:then_0
      ;[1 1 1] BasicAnimation
      (if (Variables|Default|GetHited)
        (if (AI|Components|NavMovement|IsFalling (Variables|Character|GetCharacterMovement)) :!label _label
          ;;[1 1 1] FallingAnimation
          (Sprite|SetFlipbook (Variables|Default|GetFlipBook) (Variables|FlipBook|GetFallingFlipBook))
          (elif (not (Variables|Default|GetHited))
            ;;[1 1 1] Run/IdleAnimation
            (if (!= (Math|Vector|VectorLength (Transformation|GetVelocity)) 0.0)
              (Sprite|SetFlipbook (Variables|Default|GetFlipBook) (Variables|FlipBook|GetRunFlipBook))
              (else
                (Sprite|SetFlipbook (Variables|Default|GetFlipBook) (Variables|FlipBook|GetIdleFlipBook))))))
        (elif (not (Variables|Default|GetAttacking?))
          (Utilities|FlowControl|Sequence
            (:then_0
              (goto _label))
            (:then_1
              ;;[1 1 1] Rotation
              (Math|Float|CompareFloat (.x (Transformation|GetVelocity)) 0.0
                (:>
                  (Pawn|SetControlRotation (AI|GetAIController self) (Math|Rotator|MakeRotator 0.0 0.0 0.0)))
                (:<
                  (Pawn|SetControlRotation (AI|GetAIController self) (Math|Rotator|MakeRotator 0.0 0.0 1.8e+02)))))))))
    (:then_1
      (Transformation|SetActorLocation (Math|Vector|MakeVector 0.0 (.y _returnvalue) (.z _returnvalue)) false false))))

(fn ConstructionScript)