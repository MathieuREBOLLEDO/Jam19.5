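; Flying AI enemy, drawn with a flipbook, that runs a melee attack against the player.
; Attack waits a short random time, then box-traces for pawns ahead, setting Attacking and the attack flipbook on a hit.
; A larger second trace that finds BP_Player prints a debug HIT without applying damage, and holds the blackboard "Attacking?" key true for the animation delay.
; BeginPlay stores the flipbook's starting location.
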(event EventBeginPlay
  (|CallParentFunction)
  (Variables|Default|SetInitLocation (Transformation|GetWorldLocation (Variables|Default|GetFlipBook))))

(event Collision|EventActorBeginOverlap
  (params (OtherActor :type Actor%20Object%20Reference)))

(event EventTick
  (params (DeltaSeconds :type Float%20%28single-precision%29))
  (|CallParentFunction DeltaSeconds) ; This node is disabled and will not be called.\nDrag off pins to build functionality.
)

(event EventAttack
  (bind _flipbook (Variables|Default|GetFlipBook))
  (bind _flipbook_2 (Variables|Default|GetFlipBook))
  (bind _returnvalue (Math|Vector|GetForwardVector _flipbook_2))
  (bind _returnvalue_2 (Transformation|GetWorldLocation _flipbook_2))
  (bind _returnvalue_3 (Math|Vector|GetForwardVector _flipbook))
  (bind _returnvalue_4 (Transformation|GetWorldLocation _flipbook))
  (bind _returnvalue_5 (* _returnvalue 3e+01))
  (bind _returnvalue_6 (* _returnvalue_3 3e+01))
  (bind _returnvalue_7 (+ _returnvalue_2 _returnvalue_5))
  (bind _returnvalue_8 (+ _returnvalue_4 _returnvalue_6))
  ;[1 1 1] AttackLogic
  (Utilities|FlowControl|Delay (Math|Random|RandomFloatinRange 0.2 0.5))
  (bind _outhit (Class|KismetSystemLibrary|BoxTraceSingleforObjects _returnvalue_8 _returnvalue_8 "20.000000,20.000000,20.000000" "0, 0, 0" (Utilities|Array|MakeArray "ObjectTypeQuery3") false 0 "Persistent" true))
  (if (.bBlockingHit (Collision|BreakHitResult _outhit))
    (Variables|Default|SetAttacking? true)
    (Sprite|SetFlipbook (Variables|Default|GetFlipBook) (Variables|Default|GetAttackFlipBook))
    (bind _outhit_2 (Class|KismetSystemLibrary|BoxTraceSingleforObjects _returnvalue_7 _returnvalue_7 "40.000000,40.000000,40.000000" "0, 0, 0" (Utilities|Array|MakeArray "ObjectTypeQuery3") false 0 "ForDuration" true))
    (if (.bblockinghit _outhit_2)
      (Utilities|Casting|CastToBP_Player (.hitactor _outhit_2))
      (Development|PrintString "HIT" true true "(R=0.000000,G=0.660000,B=1.000000,A=1.000000)" 5.0)
      (AI|Components|Blackboard|SetValueasBool (AI|GetBlackboard (Pawn|GetController)) (Utilities|Name|MakeLiteralName "Attacking?") true)
      (Utilities|FlowControl|Delay (Variables|Default|GetDelay%20Attack%20Animation))
      (Variables|Default|SetAttacking? false)
      (AI|Components|Blackboard|SetValueasBool (AI|GetBlackboard (Pawn|GetController)) (Utilities|Name|MakeLiteralName "Attacking?") false))))

(fn ConstructionScript
  (|CallParentFunction))