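; BP_Spawner_Manager runs escalating enemy waves, spawning random mobs at a random Y offset from the player.
; A custom ForLoopRate macro uses Delay to space out each wave's spawns.
; When spawning ends it resets a DoOnce, which Tick fires once no BP_IAMaster actors remain.
; That shows a WG_New_Card widget, scales spawn count and delay by multipliers, and starts the next wave.
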(event EventBeginPlay
  (bind _returnvalue (Game|GetPlayerCharacter 0))
  (bind _listofmobs (Variables|Default|GetListOfMobs))
  (bind _leftright (Variables|Default|GetLeftRight))
  (bind _outitem (Utilities|Array|Random _listofmobs))
  (bind _outitem_2 (Utilities|Array|Random _leftright))
  (bind _returnvalue_2 (Transformation|GetActorLocation _returnvalue))
  (bind _returnvalue_3 (+ _returnvalue_2 (Math|Vector|MakeVector 0.0 _outitem_2 0.0)))
  ;[1 1 1] Comment
  (Utilities|ForLoopRate 0 (Variables|Default|GetSpawnNumber) (Variables|Default|GetSpawnRate)
    (:LoopBody
      (if (Utilities|IsValidClass _outitem)
        (Game|SpawnActorfromClass _outitem (Math|Transform|MakeTransform _returnvalue_3 (Math|Rotator|FindLookatRotation _returnvalue_3 _returnvalue_2)) "AdjustIfPossibleButAlwaysSpawn" 0 0)))
    (:Completed
      (Utilities|FlowControl|DoOnce false) ; enters at Reset
    )))

(event EventTick
  (params (DeltaSeconds :type Float%20%28single-precision%29))
  (bind _returnvalue (Game|GetPlayerCharacter 0))
  (bind _listofmobs (Variables|Default|GetListOfMobs))
  (bind _leftright (Variables|Default|GetLeftRight))
  (bind _outitem (Utilities|Array|Random _listofmobs))
  (bind _outitem_2 (Utilities|Array|Random _leftright))
  (bind _returnvalue_2 (Transformation|GetActorLocation _returnvalue))
  (bind _returnvalue_3 (+ _returnvalue_2 (Math|Vector|MakeVector 0.0 _outitem_2 0.0)))
  (bind _outactors (Actor|GetAllActorsOfClass "/Game/Root/GD/IA/BP_IAMaster.BP_IAMaster_C"))
  (if (== (Utilities|Array|Length _outactors) 0)
    (Utilities|FlowControl|DoOnce false :!label _label
      (:Completed
        (bind _returnvalue_4 (UserInterface|CreateWidget "/Game/UI/WG_New_Card.WG_New_Card_C" (Game|GetPlayerController 0)))
        (UserInterface|Viewport|AddtoViewport _returnvalue_4 0)
        (Variables|Default|SetSpawnNumber (Math|Float|Round (* (Variables|Default|GetSpawnNumber) (Variables|Default|GetSpawnNumberMultiplier))))
        (Variables|Default|SetSpawnRate (* (Variables|Default|GetSpawnRate) (Variables|Default|GetSpawnRateMulitplier)))
        ;[1 1 1] Comment
        (Utilities|ForLoopRate 0 (Variables|Default|GetSpawnNumber) (Variables|Default|GetSpawnRate)
          (:LoopBody
            (if (Utilities|IsValidClass _outitem)
              (Game|SpawnActorfromClass _outitem (Math|Transform|MakeTransform _returnvalue_3 (Math|Rotator|FindLookatRotation _returnvalue_3 _returnvalue_2)) "AdjustIfPossibleButAlwaysSpawn" 0 0)))
          (:Completed
            (goto _label Reset)))))))

(fn ConstructionScript)