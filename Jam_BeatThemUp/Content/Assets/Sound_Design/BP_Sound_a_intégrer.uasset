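; Central audio Blueprint exposing custom events that play sound effects for card spells, enemy, player and wave events, plus music for menu, level and combo ranks.
; Family-combo reward pitch rises with combo count, capping at a triple hit; rat death loops on a delay with random pitch.
; Music events silence other tracks first; rank S plays a timed transition before its main track if still held, and combo end restores default music.
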(event Custom|ComboFamilleFinish
  (params (NbreCombo :type Integer))
  (bind _pas_souncombo (Variables|Default|GetPas_Souncombo))
  (bind _sfx_combo_sound_same_familiy (Variables|Default|GetSFX%20Combo_sound_same_familiy))
  (bind _returnvalue (* NbreCombo _pas_souncombo))
  (bind _returnvalue_2 (+ _returnvalue 0.8))
  ;[1 1 1] SFX
  ;;[1 0.3 0] SFX quand un combo de couleur se termine, pour indiquer la récompense
  (Audio|Components|Audio|Play _sfx_combo_sound_same_familiy 0.0)
  (if (>= _returnvalue_2 2.0)
    (Audio|Components|Audio|SetPitchMultiplier (Variables|Default|GetSFX%20Combo_sound_same_familiy) 2.0)
    (Utilities|FlowControl|Delay 0.1)
    (Audio|Components|Audio|Play (Variables|Default|GetSFX%20Combo_sound_same_familiy) 0.0)
    (Utilities|FlowControl|Delay 0.1)
    (Audio|Components|Audio|Play (Variables|Default|GetSFX%20Combo_sound_same_familiy) 0.0)
    (else
      (Audio|Components|Audio|SetPitchMultiplier _sfx_combo_sound_same_familiy _returnvalue_2)
      (Utilities|FlowControl|Delay 0.2))))

(event Custom|mortRat
  ;[1 1 1] SFX
  ;;[0.1197 1 0] SFX Mort d'un ennemi
  (Audio|Components|Audio|Play (Variables|Default|GetSFX%20Goblin_Death) 0.0 :!label _label)
  (Audio|Components|Audio|SetPitchMultiplier (Variables|Default|GetSFX%20Goblin_Death) (+ (* (Math|Random|RandomFloat) 0.5) 1.0))
  (Utilities|FlowControl|Delay 0.8)
  (goto _label))

(event Custom|Slash_Rat
  ;[1 1 1] SFX
  ;;[1 0.3 0] SFX Attaque d'un ennemi
  (Audio|Components|Audio|Play (Variables|Default|GetSFX%20slash_cut_ennemis) 0.0))

(event Custom|Wave_Cleared
  ;[1 1 1] SFX
  ;;[1 1 0] SFX Une Wave est finito
  (Audio|Components|Audio|Play (Variables|Default|GetSFX%20wave_cleared) 0.0))

(event Custom|Start%20Menu
  ;[1 1 1] Musiques
  ;;[0.06569 1 0.07899] Musique_Menu
  (CallFunction|ShutUpAllMusic)
  (Audio|Components|Audio|Play (Variables|Default|GetMusique_Menu_Cue) 0.0))

(event Custom|Fin%20de%20combo%20général
  ;[1 1 1] Musiques
  ;;[0.05362 1 0] Musique-Default
  (CallFunction|ShutUpAllMusic)
  (Audio|Components|Audio|Play (Variables|Default|GetMusique_sans_combo_Cue) 0.0))

(event Custom|Start_Level
  ;[1 1 1] Musiques
  ;;[0.05362 1 0] Musique-Default
  (CallFunction|ShutUpAllMusic)
  (Audio|Components|Audio|Play (Variables|Default|GetMusique_sans_combo_Cue) 0.0))

(event Custom|"Passage_lettre_C"
  ;[1 1 1] Musiques
  ;;[1 0.3 0] Musique_Combo_C
  (CallFunction|ShutUpAllMusic)
  (Audio|Components|Audio|Play (Variables|Default|GetMusique_combo_C_Cue) 0.0))

(event Custom|"Passage_Lettre_B
  ;[1 1 1] Musiques
  ;;[1 0.3 0] Musique_Combo_B
  (CallFunction|ShutUpAllMusic)
  (Audio|Components|Audio|Play (Variables|Default|GetMusique_combo_B_Cue) 0.0))

(event Custom|Passage_Lettre_A
  ;[1 1 1] Musiques
  ;;[1 0.3 0] Musique_Combo_A
  (CallFunction|ShutUpAllMusic)
  (Audio|Components|Audio|Play (Variables|Default|GetMusique_combo_A_Cue) 0.0))

(event Custom|Passage_Lettre_S
  ;[1 1 1] Musiques
  ;;[1 0.3 0] Passage_Lettre_S
  (CallFunction|ShutUpAllMusic)
  (Audio|Components|Audio|Play (Variables|Default|GetMusique_combo_S_+_transition_Cue) 0.0)
  (Utilities|FlowControl|Delay 14.62)
  (if (Variables|Default|GetTjrs_Rang_S?)
    (CallFunction|ShutUpAllMusic)
    (Audio|Components|Audio|Play (Variables|Default|GetMusique_combo_S_Cue) 0.0)))

(event Custom|Début%20de%20vague
  ;[1 1 1] SFX
  ;;[0.08618 1 0] SFX début de vague
  (Audio|Components|Audio|Play (Variables|Default|GetSFX%20Wave_Start) 0.0))

(event Custom|Shut_up_all_music
  ;[1 1 1] Musiques
  ;;[1 0 0] Arrêter toutes les musiques
  (Audio|Components|Audio|Stop (Variables|Default|GetMusique_sans_combo_Cue))
  (Audio|Components|Audio|Stop (Variables|Default|GetMusique_combo_A_Cue))
  (Audio|Components|Audio|Stop (Variables|Default|GetMusique_combo_B_Cue))
  (Audio|Components|Audio|Stop (Variables|Default|GetMusique_combo_C_Cue))
  (Audio|Components|Audio|Stop (Variables|Default|GetMusique_combo_S_+_transition_Cue))
  (Audio|Components|Audio|Stop (Variables|Default|GetMusique_combo_S_Cue))
  (Audio|Components|Audio|Stop (Variables|Default|GetMusique_Menu_Cue))
  (Audio|Components|Audio|Stop (Variables|Default|GetMusique_Transition_Cue)))

(event Custom|Mort%20du%20joueur
  ;[1 1 1] SFX
  ;;[0.4107 1 0.1214] SFX Mort Du Joueur
  (Audio|Components|Audio|Play (Variables|Default|GetSFX%20mort%20jpueur) 0.0))

(event Custom|Filler_Explosion
  ;[1 1 1] SFX
  ;;[0.09448 1 0] SFX Play_Filler_Explosion
  (Audio|Components|Audio|Play (Variables|Default|GetSFX%20Filler_Explosion) 0.0))

(event Custom|Finisher_Thunder
  ;[1 1 1] SFX
  ;;[0.09448 1 0] SFX Play_Finisher_Thunder
  (Audio|Components|Audio|Play (Variables|Default|GetSFX%20Finisher_Thunder_Rapide) 0.0))

(event Custom|Vacuum_Fire_Tornado
  ;[1 1 1] SFX
  ;;[0.09448 1 0] SFX Play_Vacuum_Fire_Tornado
  (Audio|Components|Audio|Play (Variables|Default|GetSFX%20fire_tornado) 0.0))

(event Custom|Launcher_EarthFist
  ;[1 1 1] SFX
  ;;[0.09448 1 0] SFX Play_Launcher_EarthFist
  (Audio|Components|Audio|Play (Variables|Default|GetSFX%20Launcher_RockFist) 0.0))

(event Custom|CarteGrise_Heal
  ;[1 1 1] SFX
  ;;[0.2305 1 0] SFX Play_Heal
  (Audio|Components|Audio|Play (Variables|Default|GetSFX%20heal) 0.0))

(event Custom|Carte_pas_Jouable
  ;[1 1 1] SFX
  ;;[1 1 0] SFX Le joueur essaie de jouer alors qu'il n'a pas de carte
  (Audio|Components|Audio|Play (Variables|Default|GetSFX%20Plus_de_carte) 0.0))

(fn ConstructionScript)